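; BP_TileActor is a grid tile actor that carries an index and a mesh with a randomized material.
; On BeginPlay it writes its Index as text into a WBP_GridDebug widget on its WidgetDebugger component.
; It also creates a dynamic material instance on its static mesh and sets a random OffSetTexture value, so the texture offset varies per tile.
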(event EventBeginPlay
  (bind _staticmeshcomponent (Variables|Default|GetStaticMeshComponent))
  (CallFunction|SetDebuggerText)
  (bind _returnvalue (Rendering|Material|CreateDynamicMaterialInstance _staticmeshcomponent 0 (Rendering|Material|GetMaterial _staticmeshcomponent 0) "None" :!class /Script/Engine.PrimitiveComponent))
  (Rendering|Material|SetScalarParameterValue _returnvalue "OffSetTexture" (Math|Random|RandomFloatinRange 0.0 5e+03) :!class /Script/Engine.MaterialInstanceDynamic))

(fn ConstructionScript)

(fn SetDebuggerText
  (bind _aswbp_grid_debug (Utilities|Casting|CastToWBP_GridDebug (UserInterface|GetUserWidgetObject (Variables|Default|GetWidgetDebugger))))
  (Variables|/Game/StealthGame/LevelDesign/WBP_GridDebug.WBP_GridDebug_C|SetIn%20Text _aswbp_grid_debug (Utilities|Text|FormatText "I{I}" (Variables|Default|GetIndex))))