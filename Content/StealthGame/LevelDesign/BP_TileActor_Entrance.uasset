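; Entrance tile for a procedurally built level that signals the manager to create another room and shuts its doors as the player passes through.
; Trigger boxes on both Y sides, a quick fix for 180-degree spawn rotation, close doors on overlap begin and fire the tile-activated call once on overlap end.
; Timelines animate door Z scale to close them.
; ActivateTile forces closure; the debug index label function is never run.
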(event OnComponentBeginOverlap(TriggerBox_-Y)
  (params (OverlappedComponent :type Primitive%20Component%20Object%20Reference) (OtherActor :type Actor%20Object%20Reference) (OtherComp :type Primitive%20Component%20Object%20Reference) (OtherBodyIndex :type Integer) (bFromSweep :type Boolean) (SweepResult :type Hit%20Result%20Structure%20%28by%20ref%29))
  ;[0 0 0 1 32] Qucikfix for the problem that the connector can rotate 180 on spawn, could be fixed in the future
  (if (Actor|ActorHasTag OtherActor "Player")
    (Utilities|FlowControl|DoOnce false
      (:Completed
        (Collision|SetCollisionEnabled (Variables|Default|GetCollision_-Y) "QueryOnly")
        (Collision|SetCollisionEnabled (Variables|Default|GetTriggerBox_+Y) "NoCollision")
        (CallFunction|CloseDoor-Y)))))

(event OnComponentBeginOverlap(TriggerBox_+Y)
  (params (OverlappedComponent :type Primitive%20Component%20Object%20Reference) (OtherActor :type Actor%20Object%20Reference) (OtherComp :type Primitive%20Component%20Object%20Reference) (OtherBodyIndex :type Integer) (bFromSweep :type Boolean) (SweepResult :type Hit%20Result%20Structure%20%28by%20ref%29))
  ;[0 0 0 1 32] Qucikfix for the problem that the connector can rotate 180 on spawn, could be fixed in the future
  (if (Actor|ActorHasTag OtherActor "Player")
    (Utilities|FlowControl|DoOnce false
      (:Completed
        (Collision|SetCollisionEnabled (Variables|Default|GetCollision_+Y) "QueryOnly")
        (Collision|SetCollisionEnabled (Variables|Default|GetTriggerBox_+Y) "NoCollision")
        (CallFunction|CloseDoor+Y)))))

(event OnComponentEndOverlap(TriggerBox_+Y)
  (params (OverlappedComponent :type Primitive%20Component%20Object%20Reference) (OtherActor :type Actor%20Object%20Reference) (OtherComp :type Primitive%20Component%20Object%20Reference) (OtherBodyIndex :type Integer))
  ;[0 0 0 1 32] Qucikfix for the problem that the connector can rotate 180 on spawn, could be fixed in the future
  (if (Actor|ActorHasTag OtherActor "Player")
    (Utilities|FlowControl|DoOnce false
      (:Completed
        (Default|CallOnTileActivated) ; called on the manager to creat one more room
      ))))

(event OnComponentEndOverlap(TriggerBox_-Y)
  (params (OverlappedComponent :type Primitive%20Component%20Object%20Reference) (OtherActor :type Actor%20Object%20Reference) (OtherComp :type Primitive%20Component%20Object%20Reference) (OtherBodyIndex :type Integer))
  ;[0 0 0 1 32] Qucikfix for the problem that the connector can rotate 180 on spawn, could be fixed in the future
  (if (Actor|ActorHasTag OtherActor "Player")
    (Utilities|FlowControl|DoOnce false
      (:Completed
        (Default|CallOnTileActivated) ; called on the manager to creat one more room
      ))))

(event Custom|CloseDoor_+Y
  (bind _door__y (Variables|Default|GetDoor_+Y))
  (bind _returnvalue (Transformation|GetWorldScale _door__y))
  ;[0 0 0 1 32] Qucikfix for the problem that the connector can rotate 180 on spawn, could be fixed in the future
  (EventDispatchers|UnbindallEventsfromOnTileActivated)
  (bind _size (Timeline|Timeline_0 Play)
    (:Update
      (Transformation|SetWorldScale3D _door__y (Math|Vector|MakeVector (.x _returnvalue) (.y _returnvalue) _size)))))

(event Custom|CloseDoor_-Y
  (bind _door__y (Variables|Default|GetDoor_-Y))
  (bind _returnvalue (Transformation|GetWorldScale _door__y))
  ;[0 0 0 1 32] Qucikfix for the problem that the connector can rotate 180 on spawn, could be fixed in the future
  (EventDispatchers|UnbindallEventsfromOnTileActivated)
  (bind _size (Timeline|Timeline Play)
    (:Update
      (Transformation|SetWorldScale3D _door__y (Math|Vector|MakeVector (.x _returnvalue) (.y _returnvalue) _size)))))

(event Custom|ForceCloseDoor
  (bind _triggerbox__y (Variables|Default|GetTriggerBox_+Y))
  (Utilities|FlowControl|Sequence
    (:then_0
      ;[0 0 0 1 32] Qucikfix for the problem that the connector can rotate 180 on spawn, could be fixed in the future
      (Utilities|FlowControl|DoOnce false
        (:Completed
          (Collision|SetCollisionEnabled (Variables|Default|GetCollision_-Y) "QueryOnly")
          (Collision|SetCollisionEnabled _triggerbox__y "NoCollision")
          (CallFunction|CloseDoor-Y))))
    (:then_1
      (Utilities|FlowControl|DoOnce false) ; enters at Reset
    )
    (:then_2
      (CallFunction|CloseDoor-Y))
    (:then_3
      (CallFunction|CloseDoor+Y))))

(event EventActivateTile
  (CallFunction|ForceCloseDoor))

(fn ConstructionScript)

(fn SetDebuggerText
  (bind _aswbp_grid_debug (Utilities|Casting|CastToWBP_GridDebug (UserInterface|GetUserWidgetObject (Variables|Default|GetWidgetDebugger))))
  (Variables|/Game/StealthGame/LevelDesign/WBP_GridDebug.WBP_GridDebug_C|SetIn%20Text _aswbp_grid_debug (Utilities|Text|FormatText "I{I}" (Variables|Default|GetIndex))))