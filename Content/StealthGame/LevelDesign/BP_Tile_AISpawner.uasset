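; BP_Tile_AISpawner is a level tile spawner that places enemy AI at its arrow and respawns them after they die.
; It spawns after a randomized initial delay, then binds each AI's stats-component death event to schedule a randomized respawn.
; RoomNumber picks the class: none in the first rooms, melee up to room 10, then randomly melee or shooter, unless a debug class overrides it.
; Destroying the spawner kills all its spawned AI.
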(event Custom|AIHasDied
  (Utilities|FlowControl|Delay (Math|Random|RandomFloatinRange (Variables|Default|GetMinTimeToReSpawn) (Variables|Default|GetMaxTimeToReSpawn)))
  (CallFunction|SpawnAI))

(event EventBeginPlay
  (bind _initialspawndelay (Variables|Default|GetInitialSpawnDelay))
  (|CallParentFunction)
  (Utilities|FlowControl|Delay (Math|Random|RandomFloatinRange _initialspawndelay (+ _initialspawndelay 1.0)))
  (CallFunction|SpawnAI)
  ;[1 1 1] make sure the spawned actors are destroyed too after the spawned is destroyed
  (Game|BindEventtoOnDestroyed (EventDispatchers|CreateEvent :!event KillALLSpawnedAI)))

(event EventTick
  (params (DeltaSeconds :type Float%20%28single-precision%29)))

(fn ConstructionScript
  (|CallParentFunction))

(fn SpawnAI
  (bind _aitospawndebug (Variables|Default|GetAIToSpawnDebug))
  (bind _sortedaiout (CallFunction|SortEnemytoSpawn))
  (if (Utilities|IsValidClass (select (Utilities|IsValidClass _aitospawndebug) _aitospawndebug _sortedaiout))
    (bind _returnvalue (Game|SpawnActorfromClass (select (Utilities|IsValidClass _aitospawndebug) _aitospawndebug _sortedaiout) (Transformation|GetWorldTransform (Variables|Default|GetSpawnArrow)) "Undefined" "MultiplyWithRoot" 0 0))
    (Utilities|Array|Add (Variables|Default|GetSpawnedAIs) _returnvalue)
    (EventDispatchers|BindEventtoOnDeath (Actor|GetComponentbyClass _returnvalue "/Script/MentoramaCPP5.CharacterStatsComponent") (EventDispatchers|CreateEvent :!event Custom|AIHasDied))))

(fn KillALLSpawnedAI
  (params (DestroyedActor :type Actor%20Object%20Reference))
  (for _array_element (Variables|Default|GetSpawnedAIs)
    (Actor|SetLifeSpan _array_element 3.0)
    (if (Variables|/Script/MentoramaCPP5.CharacterStatsComponent|GetIsAlive (Actor|GetComponentbyClass _array_element "/Script/MentoramaCPP5.CharacterStatsComponent"))
      (Class|CharacterStatsComponent|Die (Actor|GetComponentbyClass _array_element "/Script/MentoramaCPP5.CharacterStatsComponent")))))

(fn SortEnemytoSpawn
  (bind _roomnumber (Variables|Default|GetRoomNumber))
  (if (> (Variables|Default|GetRoomNumber) 1)
    ;[1 1 1] this will increase the probabilities of sort the shooter NPC every 10 rooms
    (if (> (Variables|Default|GetRoomNumber) 10)
      (if (> (Math|Random|RandomIntegerinRange 0 _roomnumber) (/ _roomnumber 2))
        (LocalVariables|SetSortedAI "/Game/StealthGame/Characters/AI/BP_AIChar_BTBased_Shooter.BP_AIChar_BTBased_Shooter_C")
        (else
          (LocalVariables|SetSortedAI "/Game/StealthGame/Characters/AI/BP_AIChar_BTBased_Melee.BP_AIChar_BTBased_Melee_C" :!label _label)))
      (else
        (goto _label)))
    (else
      (LocalVariables|SetSortedAI 0) ; lets not spawn in the room 0
    ))
  (return (LocalVariables|GetSortedAI)))