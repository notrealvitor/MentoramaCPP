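; Exit tile actor for the stealth game's level grid, currently mostly stubbed out.
; BeginPlay, ActivateTile, CloseDoor and the construction script are empty.
; Disconnected leftover nodes would close the door by setting collision to query-only and scaling the door's Z through a timeline, or print the tile's rotation.
; SetDebuggerText is the only working logic, writing the tile Index into its WBP_GridDebug widget.
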(event Custom|CloseDoor)

(event EventActivateTile)

(event EventBeginPlay)

(fn ConstructionScript)

(fn SetDebuggerText
  (bind _aswbp_grid_debug (Utilities|Casting|CastToWBP_GridDebug (UserInterface|GetUserWidgetObject (Variables|Default|GetWidgetDebugger))))
  (Variables|/Game/StealthGame/LevelDesign/WBP_GridDebug.WBP_GridDebug_C|SetIn%20Text _aswbp_grid_debug (Utilities|Text|FormatText "I{I}" (Variables|Default|GetIndex))))