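; Stealth-game AI enemy character, named as Behavior Tree-based, exposing melee, projectile shooting, turn-to-target and alert exclamation actions.
; Point damage triggers blood, hit montage and stun, with 5x headshot damage through CharacterStats.
; An in-range weapon interaction performs a stealth kill, and death ragdolls the mesh with a damage-scaled impulse.
; Spawns and deaths increment the game instance view model's currency fields, used as total and kill counters.
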(event OnComponentBeginOverlap(MeleeCollisionBox)
  (params (OverlappedComponent :type Primitive%20Component%20Object%20Reference) (OtherActor :type Actor%20Object%20Reference) (OtherComp :type Primitive%20Component%20Object%20Reference) (OtherBodyIndex :type Integer) (bFromSweep :type Boolean) (SweepResult :type Hit%20Result%20Structure%20%28by%20ref%29))
  ;[0 0 0] ApplyDamageToPlayer
  (if (Math|Boolean|ANDBoolean (!= OtherActor self) (!= OtherActor (Game|GetInstigator)) (Utilities|IsValid (Actor|GetComponentbyClass OtherActor "/Script/MentoramaCPP5.CharacterStatsComponent")))
    (Game|Damage|ApplyPointDamage OtherActor (Variables|Default|GetBase%20Damage) (Math|Vector|GetUnitDirection(Vector) (Transformation|GetActorLocation OtherActor) (Transformation|GetActorLocation (Game|GetInstigator))) SweepResult (Game|GetInstigatorController) self "/Script/Engine.DamageType")
    (Collision|SetCollisionEnabled (Variables|Default|GetMeleeCollisionBox) "NoCollision")))

(event Custom|Die
  (bind _mesh (Variables|Character|GetMesh))
  ;[0 0 0 1 38] Die
  (Utilities|FlowControl|DoOnce false
    (:Completed
      ;;[0.1615 0 0] increase kill, could changed to a more generic like GameplayValue_01
      (Math|Integer|IncrementInt (Variables|/Script/MentoramaCPP5.NotPlayerProperties|GetCurrentCurrency (Variables|Default|GetVM%20Not%20Player%20Properties))
        (:%20%20
          (Components|DestroyComponent (Variables|Default|GetExclamation))
          (Physics|SetSimulatePhysics _mesh true)
          (Collision|SetCollisionResponsetoChannel _mesh "ECC_Visibility" "ECR_Ignore")
          (Collision|SetCollisionEnabled (Variables|Default|GetCapsuleComponent) "NoCollision")
          (Physics|AddRadialImpulse _mesh (Variables|Default|GetHitLocation) 25.0 (* (Variables|Default|GetFinalDamage) 6e+01) "RIF_Constant" true)
          (if (Variables|Default|GetHeadshotKill)
            (Niagara|SpawnSystemAttached "/Game/StealthGame/NE_BloodFountain.NE_BloodFountain" (Variables|Character|GetMesh) "neck_01" "0, 0, 0" "0, 0, 0" "KeepRelativeOffset" true)))))))

(event Custom|LookAtPlayer
  (params (Target :type Vector%20%28by%20ref%29))
  (bind _returnvalue (Transformation|GetActorLocation))
  (bind _returnvalue_2 (Transformation|GetActorRotation))
  (bind _returnvalue_3 (Math|Rotator|FindLookatRotation _returnvalue Target))
  ;[0 0 0 1 42] LookAtPlayer (need test)
  (Timeline|Timeline PlayFromStart
    (:Update
      (Transformation|SetActorRotation (Math|Rotator|Lerp(Rotator) _returnvalue_2 _returnvalue_3 0.1 true))
      (if (Utilities|Operators|EqualEqual _returnvalue_2 _returnvalue_3 0.1)
        (Timeline|Timeline Stop)))))

(event Custom|SpotAlertVisibility
  (params (bNewVisibility :type Boolean))
  ;[0 0 0 1 42] Exclamation Spot Visibility
  (Rendering|SetVisibility (Variables|Default|GetExclamation) bNewVisibility false))

(event Custom|MeleeAttack
  (if (and (Variables|/Script/MentoramaCPP5.CharacterStatsComponent|GetIsAlive (Variables|Default|GetCharacterStats)) (Variables|/Script/MentoramaCPP5.CharacterStatsComponent|GetIsAlive (Actor|GetComponentbyClass (Game|Player|GetPlayerPawn 0) "/Script/MentoramaCPP5.CharacterStatsComponent"))) ; make sure player and this AI is alive before anything
    (Collision|SetCollisionEnabled (Variables|Default|GetMeleeCollisionBox) "QueryOnly")
    (Class|MentoramaCPP5Character|GetStunned 0.1)
    (Animation|Montage|PlayMontage (Variables|Character|GetMesh) "/Game/StealthGame/Anims/AM_SwingBack.AM_SwingBack"
      (:OnCompleted
        _)
      (:OnInterrupted
        _))
    (Collision|SetCollisionEnabled (Variables|Default|GetMeleeCollisionBox) "NoCollision")))

(event EventInteractionAction
  (params (Interactor :type Actor%20Object%20Reference) (InteractorItem :type Item%20Slot%20Object%20Reference))
  ;[0 0 0 1 38] OnInteraction
  (Utilities|IsValid Interactor
    (:Is%20Valid
      (Utilities|IsValid InteractorItem
        (:Is%20Valid
          (switch Utilities|FlowControl|Switch|SwitchonEItemType (Variables|/Script/MentoramaCPP5.ItemSlot|GetE_ItemType InteractorItem)
            (:Weapon
              (if (< (Transformation|GetDistanceTo Interactor) (Variables|Default|GetRangeToInteract))
                (Utilities|FlowControl|DoOnce false
                  (:Completed
                    (CallFunction|Die)))))))))))

(event EventBeginPlay
  (EventDispatchers|AssignOnDeath (Variables|Default|GetCharacterStats) (EventDispatchers|CreateEvent :!event Custom|Die))
  ;[0.1927 0 0] Could change totalCurrency for a more generic name like GameplayValueTotal_01
  (bind _asmentorama_game_instance (Utilities|Casting|CastToMentoramaGameInstance (Game|GetGameInstance)))
  (Variables|Default|SetVM%20Not%20Player%20Properties (Variables|/Script/MentoramaCPP5.MentoramaGameInstance|GetVM_NotPlayerProperties _asmentorama_game_instance))
  (Math|Integer|IncrementInt (Variables|/Script/MentoramaCPP5.NotPlayerProperties|GetTotalCurrency (Variables|/Script/MentoramaCPP5.MentoramaGameInstance|GetVM_NotPlayerProperties _asmentorama_game_instance))))

(event Game|Damage|EventPointDamage
  (params (Damage :type Float%20%28single-precision%29) (DamageType :type Damage%20Type%20Object%20Reference) (HitLocation :type Vector :default "0, 0, 0") (HitNormal :type Vector :default "0, 0, 0") (HitComponent :type Primitive%20Component%20Object%20Reference) (BoneName :type Name :default "None") (ShotFromDirection :type Vector :default "0, 0, 0") (InstigatedBy :type Controller%20Object%20Reference) (DamageCauser :type Actor%20Object%20Reference) (HitInfo :type Hit%20Result%20Structure%20%28by%20ref%29))
  (bind _returnvalue (Components|ComponentHasTag HitComponent "Headshot"))
  (bind _output_get (Variables|Default|SetHitLocation (.Location (Collision|BreakHitResult HitInfo))))
  (Variables|Default|SetHeadshotKill _returnvalue)
  (Niagara|SpawnSystemAttached "/Game/StealthGame/NE_BloodSplash.NE_BloodSplash" (Variables|Character|GetMesh) "root" "0, 0, 0" "0, 0, 0" "KeepRelativeOffset" true)
  (Animation|Montage|PlayMontage (Variables|Character|GetMesh) "/Game/StealthGame/Anims/AM_GeneralHitFeel.AM_GeneralHitFeel"
    (:then
      (Class|MentoramaCPP5Character|GetStunned 0.2)
      (bind _output_get_2 (Variables|Default|SetFinalDamage (Math|Float|SelectFloat (* Damage 5.0) Damage _returnvalue)))
      (Class|CharacterStatsComponent|TakeDamage (Variables|Default|GetCharacterStats) _output_get_2)
      (if (Variables|Default|GetHeadshotKill)
        (Development|PrintString "HEADSHOT" true true "(R=1.000000,G=0.000000,B=0.959795,A=1.000000)")))))

(fn ConstructionScript)

(fn GetInteractionDescription
  (return "STEALTH KILL"))

(fn LookatLocation
  (params (Target1 :type Vector%20%28by%20ref%29))
  (bind _returnvalue (Transformation|GetActorRotation))
  (Transformation|SetActorRotation (Math|Rotator|MakeRotator (.roll _returnvalue) (.pitch _returnvalue) (.yaw (Math|Rotator|FindLookatRotation (Transformation|GetActorLocation) Target1)))))

(fn ShootBullet
  (bind _self self)
  (if (and (Variables|/Script/MentoramaCPP5.CharacterStatsComponent|GetIsAlive (Variables|Default|GetCharacterStats)) (Variables|/Script/MentoramaCPP5.CharacterStatsComponent|GetIsAlive (Actor|GetComponentbyClass (Game|Player|GetPlayerPawn 0) "/Script/MentoramaCPP5.CharacterStatsComponent"))) ; make sure player and this AI is alive before anything
    (Game|SpawnActorfromClass "/Game/StealthGame/ItemAbilities/BP_Projectile.BP_Projectile_C" (Math|Transform|MakeTransform (+ (+ (* (Transformation|GetActorForwardVector) (Math|Conversions|ToVector(Float) 1e+01)) (Transformation|GetActorLocation)) "0.000000,0.000000,60.000000") (Math|Rotator|MakeRotator 0.0 0.0 (.yaw (Transformation|GetActorRotation))) "1.000000,1.000000,1.000000") "Undefined" "MultiplyWithRoot" _self 1.2e+03 (Variables|Default|GetBase%20Damage) _self)
    (Animation|PlayAnimMontage "/Game/StealthGame/Anims/AM_ShootingPistol.AM_ShootingPistol" 1.0 "None")
    (Audio|PlaySound2D "/Game/StarterContent/Audio/Explosion01.Explosion01" 1.0 1.0 0.0 0 0)))