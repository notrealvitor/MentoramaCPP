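; AI character for the stealth game that can alert on, turn toward and be stealth-killed by the player.
; AIBehaviourComp holds state; events toggle the exclamation marker and ease rotation toward a target through a Timeline.
; A weapon interaction within range kills it once, removing detection components and ragdolling the mesh with an impulse and blood effect.
; Health-state logic sets the same value on every branch, and sight-cone vertex code is disconnected.
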(event Custom|LookAtPlayer
  (params (Target :type Vector%20%28by%20ref%29))
  (bind _returnvalue (Transformation|GetActorLocation))
  (bind _returnvalue_2 (Transformation|GetActorRotation))
  (bind _returnvalue_3 (Math|Rotator|FindLookatRotation _returnvalue Target))
  ;[0 0 0 1 42] LookAtPlayer
  (Timeline|Timeline PlayFromStart
    (:Update
      (Transformation|SetActorRotation (Math|Rotator|Lerp(Rotator) _returnvalue_2 _returnvalue_3 0.1 true))
      (if (Utilities|Operators|EqualEqual _returnvalue_2 _returnvalue_3 0.1)
        (Timeline|Timeline Stop)))))

(event Custom|SpotAlertVisibility
  (params (bNewVisibility :type Boolean))
  ;[0 0 0 1 42] Exclamation Spot Visibility
  (Rendering|SetVisibility (Variables|Default|GetExclamation) bNewVisibility false))

(event EventBeginPlay
  ;[0 0 0 1 42] BeginPlay
  (Utilities|FlowControl|Sequence
    (:then_1
      ;;[0.151 0 0] this could go in the C++
      (switch Utilities|FlowControl|Switch|SwitchonEState (Variables|/Script/MentoramaCPP5.AIBehaviourComponent|GetE_AIState (Variables|Default|GetAIBehaviourComp))
        (:Roaming
          (Variables|Default|SetRandomizeDirection true))))))

(event EventInteractionAction
  (params (Interactor :type Actor%20Object%20Reference) (InteractorItem :type Item%20Slot%20Object%20Reference))
  (bind _mesh (Variables|Character|GetMesh))
  (Utilities|IsValid Interactor
    (:Is%20Valid
      (Utilities|IsValid InteractorItem
        (:Is%20Valid
          (switch Utilities|FlowControl|Switch|SwitchonEItemType (Variables|/Script/MentoramaCPP5.ItemSlot|GetE_ItemType InteractorItem)
            (:Weapon
              (if (< (Transformation|GetDistanceTo Interactor) (Variables|Default|GetRangeToInteract))
                (Utilities|FlowControl|DoOnce false
                  (:Completed
                    (Variables|/Script/MentoramaCPP5.AIBehaviourComponent|SetbIsAlive (Variables|Default|GetAIBehaviourComp) false)
                    (Components|DestroyComponent (Variables|Default|GetExclamation))
                    (Physics|SetSimulatePhysics _mesh true)
                    (Collision|SetCollisionResponsetoChannel _mesh "ECC_GameTraceChannel2" "ECR_Ignore")
                    (Collision|SetCollisionEnabled (Variables|Default|GetCapsuleComponent) "NoCollision")
                    (Physics|AddRadialImpulse _mesh (Transformation|GetActorLocation) 5e+02 1e+02 "RIF_Constant" true)
                    (Niagara|SpawnSystemAttached "/Game/StealthGame/NE_BloodFountain.NE_BloodFountain" (Variables|Character|GetMesh) "neck_01" "0, 0, 0" "0, 0, 0" "KeepRelativeOffset" true)))))))))))

(fn ConstructionScript)

(fn GetInteractionDescription
  (return "STEALTH KILL"))

(fn SetHealthState
  (bind _s_aidata (Variables|Default|GetS_AIData))
  (if (>= (.health _s_aidata) 6e+01)
    (Variables|Default|SetE_HealthState 0)
    (return)
    (elif (<= (.health _s_aidata) 0.0)
      (Variables|Default|SetE_HealthState 0)
      (return)
      (elif (< 0.0 3e+01)
        (Variables|Default|SetE_HealthState 0)
        (return)
        (elif (< (.health _s_aidata) 6e+01)
          (Variables|Default|SetE_HealthState 0)
          (return))))))

(fn ConvertSightPointstoVertices
  (params (SightPoints :type Array%20of%20Vectors)))

(fn PrintSelfAction
  (params (Action%20to%20Print :type String) (Duration :type Float%20%28double-precision%29))
  (Development|PrintString (Utilities|String|Append (Utilities|GetDisplayName self) " is " Action%20to%20Print) true true "(R=0.000000,G=0.660000,B=1.000000,A=1.000000)" Duration))

(fn InteractionRange
  (return 0))