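; Player character for the stealth game, handling inventory hotbar, item abilities, interaction and a UI mode toggle.
; BeginPlay builds the HUD from the GameInstance's shared viewmodel, which also supplies slot data.
; Selecting a slot attaches the item mesh to a type-based socket and constructs its primary and secondary ability objects for the action inputs.
; Dropping spawns a pickup; successful interaction plays a throat-cut montage; F adds debug items.
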(event Custom|DebugSlots
  (for _index (range 0 (- (Variables|/Script/MentoramaCPP5.InventoryComponent|GetNumberOfSlots (Variables|Default|GetInventory)) 1))
    (Utilities|IsValid (.itemslot (Class|InventoryComponent|GetSlot (Variables|Default|GetInventory) _index))
      (:Is%20Valid
        (Development|PrintText (Utilities|Text|FormatText "Slot {index} tem {amount}  de {item}" _index (.amount (Class|InventoryComponent|GetSlot (Variables|Default|GetInventory) _index)) (Variables|/Script/MentoramaCPP5.ItemSlot|GetName (.itemslot (Class|InventoryComponent|GetSlot (Variables|Default|GetInventory) _index))))))
      (:Is%20Not%20Valid
        (Development|PrintText (Utilities|Text|FormatText "Slot {index} não tem item" _index))))))

(event Input|EnhancedActionEvents|EnhancedInputActionIA_UIMode
  (params (ActionValue :type Boolean) (ElapsedSeconds :type Float%20%28double-precision%29) (TriggeredSeconds :type Float%20%28double-precision%29) (InputAction :type Input%20Action%20Object%20Reference :default "/Game/StealthGame/Input/IA_UIMode.IA_UIMode"))
  ;[0 0 0 1 74] Input
  (:Started
    (if (Variables|Default|GetUIMode)
      (CallFunction|ToggleUImode true)
      (else
        (CallFunction|ToggleUImode false)))))

(event Input|EnhancedActionEvents|EnhancedInputActionIA_Slot01
  (params (ActionValue :type Boolean) (ElapsedSeconds :type Float%20%28double-precision%29) (TriggeredSeconds :type Float%20%28double-precision%29) (InputAction :type Input%20Action%20Object%20Reference :default "/Game/StealthGame/Input/IA_Slot01.IA_Slot01"))
  ;[0 0 0 1 74] Input
  (:Started
    (CallFunction|SelectItem)))

(event Input|EnhancedActionEvents|EnhancedInputActionIA_PrimaryAction
  (params (ActionValue :type Boolean) (ElapsedSeconds :type Float%20%28double-precision%29) (TriggeredSeconds :type Float%20%28double-precision%29) (InputAction :type Input%20Action%20Object%20Reference :default "/Game/StealthGame/Input/IA_PrimaryAction.IA_PrimaryAction"))
  ;[0 0 0 1 74] Input
  (:Started
    (bind _ref_primaryabilityactive (Variables|Default|GetREF_PrimaryAbilityActive)
      (:then
        (Class|ItemAbility|TriggerAbility _ref_primaryabilityactive))
      (:else))))

(event Input|EnhancedActionEvents|EnhancedInputActionIA_SecondaryAction
  (params (ActionValue :type Boolean) (ElapsedSeconds :type Float%20%28double-precision%29) (TriggeredSeconds :type Float%20%28double-precision%29) (InputAction :type Input%20Action%20Object%20Reference :default "/Game/StealthGame/Input/IA_SecondaryAction.IA_SecondaryAction"))
  ;[0 0 0 1 74] Input
  (:Started
    (bind _ref_secondaryability (Variables|Default|GetREF_SecondaryAbility)
      (:then
        (Class|ItemAbility|TriggerAbility _ref_secondaryability))
      (:else))))

(event Input|EnhancedActionEvents|EnhancedInputActionIA_DropItem
  (params (ActionValue :type Boolean) (ElapsedSeconds :type Float%20%28double-precision%29) (TriggeredSeconds :type Float%20%28double-precision%29) (InputAction :type Input%20Action%20Object%20Reference :default "/Game/StealthGame/Input/IA_DropItem.IA_DropItem"))
  (bind _vm_not_player_properties (Variables|Default|GetVM%20Not%20Player%20Properties))
  (bind _selecteditemindex (Variables|Default|GetSelectedItemIndex))
  (bind _inventoryslots (Variables|/Script/MentoramaCPP5.NotPlayerProperties|GetInventorySlots _vm_not_player_properties))
  (bind _output (Utilities|Array|Get(acopy) _inventoryslots _selecteditemindex))
  ;[0 0 0 1 74] Input
  (CallFunction|DropItem _selecteditemindex (.itemslot _output) (.amount _output)))

(event Input|EnhancedActionEvents|EnhancedInputActionIA_Slot02
  (params (ActionValue :type Boolean) (ElapsedSeconds :type Float%20%28double-precision%29) (TriggeredSeconds :type Float%20%28double-precision%29) (InputAction :type Input%20Action%20Object%20Reference :default "/Game/StealthGame/Input/IA_Slot02.IA_Slot02"))
  ;[0 0 0 1 74] Input
  (:Started
    (CallFunction|SelectItem 1)))

(event Input|EnhancedActionEvents|EnhancedInputActionIA_Slot03
  (params (ActionValue :type Boolean) (ElapsedSeconds :type Float%20%28double-precision%29) (TriggeredSeconds :type Float%20%28double-precision%29) (InputAction :type Input%20Action%20Object%20Reference :default "/Game/StealthGame/Input/IA_Slot03.IA_Slot03"))
  ;[0 0 0 1 74] Input
  (:Started
    (CallFunction|SelectItem 2)))

(event Input|EnhancedActionEvents|EnhancedInputActionIA_Slot04
  (params (ActionValue :type Boolean) (ElapsedSeconds :type Float%20%28double-precision%29) (TriggeredSeconds :type Float%20%28double-precision%29) (InputAction :type Input%20Action%20Object%20Reference :default "/Game/StealthGame/Input/IA_Slot04.IA_Slot04"))
  ;[0 0 0 1 74] Input
  (:Started
    (CallFunction|SelectItem 3)))

(event Input|EnhancedActionEvents|EnhancedInputActionIA_Slot05
  (params (ActionValue :type Boolean) (ElapsedSeconds :type Float%20%28double-precision%29) (TriggeredSeconds :type Float%20%28double-precision%29) (InputAction :type Input%20Action%20Object%20Reference :default "/Game/StealthGame/Input/IA_Slot05.IA_Slot05"))
  ;[0 0 0 1 74] Input
  (:Started
    (CallFunction|SelectItem 4)))

(event Input|EnhancedActionEvents|EnhancedInputActionIA_Slot06
  (params (ActionValue :type Boolean) (ElapsedSeconds :type Float%20%28double-precision%29) (TriggeredSeconds :type Float%20%28double-precision%29) (InputAction :type Input%20Action%20Object%20Reference :default "/Game/StealthGame/Input/IA_Slot06.IA_Slot06"))
  ;[0 0 0 1 74] Input
  (:Started
    (CallFunction|SelectItem 5)))

(event Input|EnhancedActionEvents|EnhancedInputActionIA_Slot07
  (params (ActionValue :type Boolean) (ElapsedSeconds :type Float%20%28double-precision%29) (TriggeredSeconds :type Float%20%28double-precision%29) (InputAction :type Input%20Action%20Object%20Reference :default "/Game/StealthGame/Input/IA_Slot07.IA_Slot07"))
  ;[0 0 0 1 74] Input
  (:Started
    (CallFunction|SelectItem 6)))

(event Input|EnhancedActionEvents|EnhancedInputActionIA_Slot08
  (params (ActionValue :type Boolean) (ElapsedSeconds :type Float%20%28double-precision%29) (TriggeredSeconds :type Float%20%28double-precision%29) (InputAction :type Input%20Action%20Object%20Reference :default "/Game/StealthGame/Input/IA_Slot08.IA_Slot08"))
  ;[0 0 0 1 74] Input
  (:Started
    (CallFunction|SelectItem 7)))

(event Input|EnhancedActionEvents|EnhancedInputActionIA_Interact
  (params (ActionValue :type Boolean) (ElapsedSeconds :type Float%20%28double-precision%29) (TriggeredSeconds :type Float%20%28double-precision%29) (InputAction :type Input%20Action%20Object%20Reference :default "/Game/ThirdPerson/Input/Actions/IA_Interact.IA_Interact"))
  ;[0 0 0 1 74] Input
  (:Started
    (Class|MentoramaCPP5Character|Interact)))

(event EventBeginPlay
  (Utilities|FlowControl|Sequence
    (:then_0
      (CallFunction|LoadifValidUsername))
    (:then_1
      (bind _asgi_my_game_instance (Utilities|Casting|CastToGI_MyGameInstance (Game|GetGameInstance)))
      (bind _output_get (Variables|Default|SetVM%20Not%20Player%20Properties (Variables|/Game/Blueprints/GI_MyGameInstance.GI_MyGameInstance_C|GetVM_NotPlayerProperties _asgi_my_game_instance)))
      (bind _returnvalue (UserInterface|CreateWidget "/Game/Blueprints/Widgets/WBP_StealthPlayerHUD.WBP_StealthPlayerHUD_C" (Game|GetPlayerController 0) _output_get))
      (bind _output_get_2 (Variables|Default|SetWBP_PlayerHUD _returnvalue))
      (UserInterface|Viewport|AddtoViewport _output_get_2 0))))

(event EventInteractionSuccessful
  (Animation|Montage|PlayMontage (Variables|Character|GetMesh) "/Game/StealthGame/Anims/AM_CutThroat_v1.AM_CutThroat_v1"))

(event EventTick
  (params (DeltaSeconds :type Float%20%28single-precision%29)))

(event Input|KeyboardEvents|F
  (params (Key :type Key%20Structure :default "None"))
  (:Pressed
    (Class|InventoryComponent|AddItemtoInventory (Variables|Default|GetInventory) "/Game/StealthGame/Itens/DA_Item_Helmet.DA_Item_Helmet" 1)
    (Class|InventoryComponent|AddItemtoInventory (Variables|Default|GetInventory) "/Game/StealthGame/Itens/DA_Item_Potion.DA_Item_Potion" 2)
    (CallFunction|DebugSlots)))

(fn ConstructionScript)

(fn LoadifValidUsername)

(fn GetInteractionDescription
  (return "Player??"))

(fn ToggleUImode
  (params (OFF :type Boolean))
  (bind _returnvalue (Game|GetPlayerController 0))
  (if OFF
    (Variables|Default|SetUIMode false)
    (Variables|/Script/Engine.PlayerController|SetbShowMouseCursor _returnvalue false)
    (Input|SetInputModeGameOnly _returnvalue false)
    (else
      (Variables|Default|SetUIMode true)
      (Variables|/Script/Engine.PlayerController|SetbShowMouseCursor _returnvalue true)
      (Input|SetInputModeGameandUI _returnvalue (Variables|Default|GetWBP_PlayerHUD) "DoNotLock" true false))))

(fn DropItem
  (params (Index :type Integer) (ItemData :type Item%20Slot%20Object%20Reference) (Amount :type Integer))
  (bind _inventory (Variables|Default|GetInventory))
  (Utilities|IsValid ItemData
    (:Is%20Valid
      (Game|SpawnActorfromClass "/Game/StealthGame/Itens/BP_PickUpBase.BP_PickUpBase_C" (Math|Transform|MakeTransform (+ (Transformation|GetActorLocation) (* (Transformation|GetActorForwardVector) (Math|Conversions|ToVector(Float) 100))) "0, 0, 0" "1.000000,1.000000,1.000000") "Undefined" "MultiplyWithRoot" 0 ItemData Amount 0)
      (Class|InventoryComponent|ClearSlot _inventory Index)
      (Class|InventoryComponent|UpdateVisualModel _inventory)
      (Variables|Default|SetSelectedItemSlot 0)
      (CallFunction|UpdateSelectedItemAttachment "None"))))

(fn SelectItem
  (params (SlotIndex :type Integer))
  (Default|SelectSlotbyIndex (Variables|/Game/Blueprints/Widgets/WBP_StealthPlayerHUD.WBP_StealthPlayerHUD_C|GetWBP_InventoryBar (Variables|Default|GetWBP_PlayerHUD)) SlotIndex)
  (Variables|Default|SetSelectedItemIndex SlotIndex)
  (bind _output_get (Variables|Default|SetSelectedItemSlot (.itemslot (Utilities|Array|Get(acopy) (Variables|/Script/MentoramaCPP5.NotPlayerProperties|GetInventorySlots (Variables|Default|GetVM%20Not%20Player%20Properties)) SlotIndex))))
  (Utilities|IsValid _output_get
    (:Is%20Valid
      (CallFunction|UpdateSelectedItemAttachment (Utilities|Select :Index (Variables|/Script/MentoramaCPP5.ItemSlot|GetE_ItemType _output_get) :Weapon "hand_rSocket" :Throwable "hand_rSocket" :Consumable "hand_rSocket" :Equipment "headSocket"))
      (Utilities|FlowControl|Sequence
        (:then_0
          (if (Utilities|IsValidClass (Variables|/Script/MentoramaCPP5.ItemSlot|GetItemSecondaryAbility (Variables|Default|GetSelectedItemSlot)))
            (bind _returnvalue (Game|ConstructObjectfromClass (Variables|/Script/MentoramaCPP5.ItemSlot|GetItemSecondaryAbility (Variables|Default|GetSelectedItemSlot))))
            (Variables|Default|SetREF_SecondaryAbility _returnvalue)
            (else
              (Variables|Default|SetREF_SecondaryAbility 0))))
        (:then_1
          (if (Utilities|IsValidClass (Variables|/Script/MentoramaCPP5.ItemSlot|GetItemPrimaryAbility (Variables|Default|GetSelectedItemSlot)))
            (bind _returnvalue_2 (Game|ConstructObjectfromClass (Variables|/Script/MentoramaCPP5.ItemSlot|GetItemPrimaryAbility (Variables|Default|GetSelectedItemSlot))))
            (Variables|Default|SetREF_PrimaryAbilityActive _returnvalue_2)
            (else
              (Variables|Default|SetREF_PrimaryAbilityActive 0))))))
    (:Is%20Not%20Valid
      (CallFunction|UpdateSelectedItemAttachment "None")
      (Variables|Default|SetREF_PrimaryAbilityActive 0)
      (Variables|Default|SetREF_SecondaryAbility 0))))

(fn UpdateSelectedItemAttachment
  (params (SocketName :type Name))
  (bind _attachedmeshactor (Variables|Default|GetAttachedMeshActor)
    (:then
      (Actor|DestroyActor _attachedmeshactor)
      (Variables|Default|SetAttachedMeshActor 0))
    (:else
      _))
  (bind _selecteditemslot (Variables|Default|GetSelectedItemSlot)
    (:then
      (bind _returnvalue (Game|SpawnActorfromClass "/Game/StealthGame/Itens/BP_HandItemBase.BP_HandItemBase_C" (Math|Transform|MakeTransform "0, 0, 0" "0, 0, 0" "1.000000,1.000000,1.000000") "Undefined" "MultiplyWithRoot" 0 (select (Utilities|IsValid (Variables|/Script/MentoramaCPP5.ItemSlot|GetMesh _selecteditemslot)) (Variables|/Script/MentoramaCPP5.ItemSlot|GetMesh _selecteditemslot) 0) 0))
      (bind _output_get (Variables|Default|SetAttachedMeshActor _returnvalue))
      (Transformation|AttachComponentToComponent _output_get (Variables|Character|GetMesh) SocketName "KeepRelative" "KeepRelative" "KeepRelative" true))
    (:else)))