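; BP_MeleeCollisionBox is a melee hitbox actor that deals point damage to what it overlaps.
; On overlap, it ignores itself and its instigator, then applies damage credited to the instigator's controller.
; The hit direction points from the victim toward the instigator, and the rebuilt sweep result uses the box actor's location.
; Collision switches off after the first valid hit, followed by a debug print.
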(event OnComponentBeginOverlap(CustomCollisionBox)
  (params (OverlappedComponent :type Primitive%20Component%20Object%20Reference) (OtherActor :type Actor%20Object%20Reference) (OtherComp :type Primitive%20Component%20Object%20Reference) (OtherBodyIndex :type Integer) (bFromSweep :type Boolean) (SweepResult :type Hit%20Result%20Structure%20%28by%20ref%29))
  (bind (_bblockinghit _binitialoverlap _time _distance _location _impactpoint _normal _impactnormal _physmat _hitactor _hitcomponent _hitbonename _bonename _hititem _elementindex _faceindex _tracestart _traceend) (Collision|BreakHitResult SweepResult))
  (if (and (!= OtherActor self) (!= OtherActor (Game|GetInstigator)))
    (Game|Damage|ApplyPointDamage OtherActor (Variables|Default|GetBaseDamage) (Math|Vector|GetUnitDirection(Vector) (Transformation|GetActorLocation OtherActor) (Transformation|GetActorLocation (Game|GetInstigator))) (Collision|MakeHitResult _bblockinghit _binitialoverlap _time _distance (Transformation|GetActorLocation) _impactpoint _normal _impactnormal _physmat _hitactor _hitcomponent _hitbonename _bonename _hititem _elementindex _faceindex _tracestart _traceend) (Game|GetInstigatorController) self "/Script/Engine.DamageType")
    (Collision|SetCollisionEnabled (Variables|Default|GetCustomCollisionBox) "NoCollision")
    (Development|PrintString "HITY")))

(event EventBeginPlay)

(fn ConstructionScript)