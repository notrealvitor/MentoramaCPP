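; BP_Bullet is a bullet actor that deals point damage to the first actor its Box overlaps, ignoring itself and its instigator.
; A DoOnce gate limits it to one hit, passing the sweep result and a hit direction that points from the victim toward the instigator.
; After the hit it hides the mesh, deactivates the Niagara effect and sets a short life span instead of destroying itself immediately.
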(event OnComponentBeginOverlap(Box)
  (params (OverlappedComponent :type Primitive%20Component%20Object%20Reference) (OtherActor :type Actor%20Object%20Reference) (OtherComp :type Primitive%20Component%20Object%20Reference) (OtherBodyIndex :type Integer) (bFromSweep :type Boolean) (SweepResult :type Hit%20Result%20Structure%20%28by%20ref%29))
  (if (and (!= OtherActor self) (!= OtherActor (Game|GetInstigator)))
    (Utilities|FlowControl|DoOnce false
      (:Completed
        (Game|Damage|ApplyPointDamage OtherActor (Variables|Default|GetBase%20Damage) (Math|Vector|GetUnitDirection(Vector) (Transformation|GetActorLocation OtherActor) (Transformation|GetActorLocation (Game|GetInstigator))) SweepResult 0 self "/Script/Engine.DamageType")
        (Development|SetHiddeninGame (Variables|Default|GetStaticMesh) true false)
        (Components|Activation|Deactivate (Variables|Default|GetNiagara))
        (Actor|SetLifeSpan 2.0)))))

(event EventBeginPlay)

(event Collision|EventActorBeginOverlap
  (params (OtherActor :type Actor%20Object%20Reference)))

(event EventTick
  (params (DeltaSeconds :type Float%20%28single-precision%29)))

(fn ConstructionScript)