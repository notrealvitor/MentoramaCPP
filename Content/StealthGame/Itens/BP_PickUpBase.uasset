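; Base pickup actor that adds an item to the interacting actor's inventory.
; An ItemData reference supplies the mesh set in the construction script and the name used in the "pick up" interaction prompt.
; On interaction it passes ItemData and Amount to the interactor's InventoryComponent and destroys itself only if the add succeeds.
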(event EventInteractionAction
  (params (Interactor :type Actor%20Object%20Reference) (InteractorItem :type Item%20Slot%20Object%20Reference))
  (bind _itemdata (Variables|Default|GetItemData))
  (Utilities|IsValid _itemdata
    (:Is%20Valid
      (bind _returnvalue (Class|InventoryComponent|AddItemtoInventory (Actor|GetComponentbyClass Interactor "/Script/MentoramaCPP5.InventoryComponent") _itemdata (Variables|Default|GetAmount)))
      (if _returnvalue
        (Actor|DestroyActor)))))

(fn ConstructionScript
  (bind _itemdata (Variables|Default|GetItemData)
    (:then
      (Components|StaticMesh|SetStaticMesh (Variables|Default|GetStaticMesh) (Variables|/Script/MentoramaCPP5.ItemSlot|GetMesh _itemdata)))
    (:else)))

(fn GetInteractionDescription
  (return (Utilities|Text|FormatText "pick up {itemname}" (Variables|/Script/MentoramaCPP5.ItemSlot|GetName (Variables|Default|GetItemData)))))