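; Healing station actor that restores health to characters standing inside its sphere.
; Sphere overlap events add and remove MentoramaCPP5Character actors in a CharactersInside list.
; A Delay on Tick throttles healing to about once per second, applying a fixed amount through each CharacterStatsComponent and printing a debug message.
; For AI-controlled characters, it also has the AIC_BPBaseBTController push updated health to the Blackboard.
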(event OnComponentBeginOverlap(Sphere)
  (params (OverlappedComponent :type Primitive%20Component%20Object%20Reference) (OtherActor :type Actor%20Object%20Reference) (OtherComp :type Primitive%20Component%20Object%20Reference) (OtherBodyIndex :type Integer) (bFromSweep :type Boolean) (SweepResult :type Hit%20Result%20Structure%20%28by%20ref%29))
  (bind _asmentorama_cpp5character (Utilities|Casting|CastToMentoramaCPP5Character OtherActor))
  (Utilities|Array|AddUnique (Variables|Default|GetCharactersInside) _asmentorama_cpp5character))

(event OnComponentEndOverlap(Sphere)
  (params (OverlappedComponent :type Primitive%20Component%20Object%20Reference) (OtherActor :type Actor%20Object%20Reference) (OtherComp :type Primitive%20Component%20Object%20Reference) (OtherBodyIndex :type Integer))
  (bind _asmentorama_cpp5character (Utilities|Casting|CastToMentoramaCPP5Character OtherActor))
  (Utilities|Array|RemoveItem (Variables|Default|GetCharactersInside) _asmentorama_cpp5character))

(event EventBeginPlay)

(event Collision|EventActorBeginOverlap
  (params (OtherActor :type Actor%20Object%20Reference)))

(event EventTick
  (params (DeltaSeconds :type Float%20%28single-precision%29))
  (bind _returnvalue (Math|Float|MakeLiteralFloat 1e+01))
  (Utilities|FlowControl|Delay 1.0)
  (for _array_element (Variables|Default|GetCharactersInside)
    (Class|CharacterStatsComponent|Heal (Actor|GetComponentbyClass _array_element "/Script/MentoramaCPP5.CharacterStatsComponent") _returnvalue)
    (Development|PrintString (Utilities|String|Append "Healing " (Utilities|GetDisplayName _array_element) " + " (Utilities|String|ToString(Float) _returnvalue) " ----- " (Utilities|String|ToString(Float) (Variables|/Script/MentoramaCPP5.CharacterStatsComponent|GetHealth (Actor|GetComponentbyClass _array_element "/Script/MentoramaCPP5.CharacterStatsComponent")))) true true "(R=0.011136,G=1.000000,B=0.000000,A=1.000000)" 1.0)
    (Utilities|IsValid (AI|GetAIController _array_element)
      (:Is%20Valid
        (bind _asaic_bpbase_btcontroller (Utilities|Casting|CastToAIC_BPBaseBTController (AI|GetAIController _array_element)))
        (Default|UpdateHealthtoBB _asaic_bpbase_btcontroller)))))

(fn ConstructionScript)