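; Game mode Blueprint that runs a level's win, defeat, restart and quit flow for a stealth game.
; On BeginPlay it feeds the collectible total into the game instance's non-player ViewModel, then updates map time on Tick while playing.
; Bound end-game events stop play, swap the HUD for a result widget and enter menu mode.
; Restart resets the ViewModel and reopens the level; quit uses a confirmation modal; checkpoint enabling is unused.
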(event Custom|OnNoButtonReleased_EventNo
  ;[0 0 0 1 42] QuitGame Modal
  (Widget|RemovefromParent (stale Custom|CreateQuitGameConfirmationModal _returnvalue))
  (CallFunction|UnbindAllfromModalConfirm (stale Custom|CreateQuitGameConfirmationModal _returnvalue)))

(event Custom|OnMyGameWon_Event
  (if (Variables|Default|GetbGamePlaying)
    (Variables|Default|SetbGamePlaying false)
    (bind _outputwidget (CallFunction|ReplaceCurrentWidget "/Game/Blueprints/Widgets/WBP_ScoreScreen.WBP_ScoreScreen_C"))
    (Variables|/Game/Blueprints/Widgets/WBP_ScoreScreen.WBP_ScoreScreen_C|SetNotPlayerProperties (.AsWBP%20Score%20Screen (Utilities|Casting|CastToWBP_ScoreScreen _outputwidget)) (Variables|/Game/Blueprints/GI_MyGameInstance.GI_MyGameInstance_C|GetVM_NotPlayerProperties (.AsGI%20My%20Game%20Instance (Utilities|Casting|CastToGI_MyGameInstance (Game|GetGameInstance)))))
    (CallFunction|SetControllertoMenuMode)))

(event Custom|UnbindAllFromModalConfirm
  (params (Target :type WBP%20Modal%20Confirm%20Object%20Reference))
  ;[0 0 0 1 42] QuitGame Modal
  (EventDispatchers|UnbindallEventsfromOnNoButtonReleased Target)
  (EventDispatchers|UnbindallEventsfromOnYesButtonReleased Target))

(event Custom|OnMyGameOver_Event
  (if (Variables|Default|GetbGamePlaying)
    (Variables|Default|SetbGamePlaying false)
    (CallFunction|ReplaceCurrentWidget "/Game/StealthGame/Widgets/WBP_DefeatScreen_MainStealth.WBP_DefeatScreen_MainStealth_C")
    (CallFunction|SetControllertoMenuMode)))

(event Custom|RestartGame
  ;[0 0 0 1 42] RestartGame
  (Input|SetInputModeGameOnly (Game|GetPlayerController 0) false)
  (CallFunction|ResetVMPlayerProperties)
  (bind _returnvalue (Game|GetCurrentLevelName true))
  (Game|OpenLevel(byName) (Utilities|String|StringToName _returnvalue)))

(event Custom|CreateQuitGameConfirmationModal
  ;[0 0 0 1 42] QuitGame Modal
  (bind _returnvalue (UserInterface|CreateWidget "/Game/Blueprints/Widgets/WBP_ModalConfirm.WBP_ModalConfirm_C"))
  (UserInterface|Viewport|AddtoViewport _returnvalue 0)
  (EventDispatchers|AssignOnNoButtonReleased _returnvalue (delegate Custom|OnNoButtonReleased_EventNo))
  (EventDispatchers|AssignOnYesButtonReleased _returnvalue (delegate Custom|OnYesButtonReleased_EventYes)))

(event Custom|OnStealthGameOver_Event
  (if (Variables|Default|GetbGamePlaying)
    (Variables|Default|SetbGamePlaying false)
    (CallFunction|ReplaceCurrentWidget "/Game/StealthGame/Widgets/WBP_DefeatScreen_Stealth_legacy.WBP_DefeatScreen_Stealth_legacy_C")
    (CallFunction|SetControllertoMenuMode)))

(event Custom|OnYesButtonReleased_EventYes
  ;[0 0 0 1 42] QuitGame Modal
  (Game|QuitGame 0 "Quit" false))

(event EventBeginPlay
  (EventDispatchers|BindEventtoOnMyGameWon (delegate Custom|OnMyGameWon_Event))
  (EventDispatchers|BindEventtoOnStealthGameOver (delegate Custom|OnStealthGameOver_Event))
  (EventDispatchers|BindEventtoOnMyGameOver (delegate Custom|OnMyGameOver_Event))
  ;[0 0 0] Get Reference to VM
  (bind _asgi_my_game_instance (Utilities|Casting|CastToGI_MyGameInstance (Game|GetGameInstance)))
  (Variables|Default|SetVM%20NotPlayer%20Properties (Variables|/Game/Blueprints/GI_MyGameInstance.GI_MyGameInstance_C|GetVM_NotPlayerProperties _asgi_my_game_instance))
  ;[0 0 0] Send the total collectionables amount in the map to the VM
  (bind _outactors (Actor|GetAllActorsOfClass "/Game/Blueprints/LevelDesign/BP_MasterCollectible.BP_MasterCollectible_C"))
  (Variables|/Game/Blueprints/Widgets/VisualModel/VM_PlayerProperties.VM_PlayerProperties_C|SetTotalCurrency (Variables|Default|GetVM%20NotPlayer%20Properties) (Utilities|Array|Length _outactors)))

(event EventTick
  (params (DeltaSeconds :type Float%20%28single-precision%29))
  (if (Variables|Default|GetbGamePlaying)
    (Variables|/Script/MentoramaCPP5.NotPlayerProperties|SetTotalMapTime (Variables|Default|GetVM%20NotPlayer%20Properties) (Utilities|Time|GetTimeSeconds))))

(fn ConstructionScript)

(fn ReplaceCurrentWidget
  (params (Class :type User%20Widget%20Class%20Reference))
  ;[0 0 0 1 26] remove the player hud
  ; (I think its better in the controller)
  (bind _wbp_playerhud (Variables|/Game/StealthGame/Characters/BP_StealthChar.BP_StealthChar_C|GetWBP_PlayerHUD (.AsBP%20Stealth%20Char (Utilities|Casting|CastToBP_StealthChar (Game|Player|GetPlayerPawn 0))))
    (:then
      (Widget|RemovefromParent _wbp_playerhud))
    (:else
      _))
  (bind _currentmenu (Variables|Default|GetCurrentMenu)
    (:then
      (Widget|RemovefromParent _currentmenu))
    (:else
      _))
  (bind _returnvalue (UserInterface|CreateWidget Class))
  (Variables|Default|SetCurrentMenu _returnvalue)
  (UserInterface|Viewport|AddtoViewport _returnvalue 0)
  (Input|SetInputModeUIOnly (Game|GetPlayerController 0) _returnvalue "DoNotLock" false)
  (return _returnvalue))

(fn SetControllertoMenuMode
  (bind _returnvalue (Game|GetPlayerController 0))
  (Variables|/Script/Engine.PlayerController|SetbShowMouseCursor _returnvalue true)
  (bind _asmy_cppcharacter (Utilities|Casting|CastToMyCPPCharacter (Game|Player|GetPlayerPawn 0)))
  (Input|DisableInput _asmy_cppcharacter _returnvalue))

(fn ResetVMPlayerProperties
  (bind _vm_notplayer_properties (Variables|Default|GetVM%20NotPlayer%20Properties))
  (Variables|/Game/Blueprints/Widgets/VisualModel/VM_PlayerProperties.VM_PlayerProperties_C|SetCurrentCurrency _vm_notplayer_properties 0)
  (Variables|/Game/Blueprints/Widgets/VisualModel/VM_PlayerProperties.VM_PlayerProperties_C|SetTotalCurrency _vm_notplayer_properties 0)
  (Variables|/Script/MentoramaCPP5.NotPlayerProperties|SetTotalMapTime _vm_notplayer_properties 0.0)
  (Variables|/Game/Blueprints/Widgets/VisualModel/VM_PlayerProperties.VM_PlayerProperties_C|SetMapResource _vm_notplayer_properties 0)
  (Class|InventoryComponent|UpdateVisualModel (Actor|GetComponentbyClass (Game|Player|GetPlayerPawn 0) "/Script/MentoramaCPP5.InventoryComponent")))

(fn EnableActiveCheckpoint
  (bind _returnvalue (SaveGame|DoesSaveGameExist "Checkpoint")) ; not being used
  (if _returnvalue
    (bind _returnvalue_2 (SaveGame|LoadGamefromSlot "Checkpoint"))
    (bind _assavebp_checkpoint (Utilities|Casting|CastToSAVEBP_Checkpoint _returnvalue_2))
    (Variables|Default|SetAs%20SAVEBP%20Checkpoint _assavebp_checkpoint)
    (else
      (bind _returnvalue_3 (SaveGame|CreateSaveGameObject "/Game/Blueprints/System/SaveGame/SAVEBP_Checkpoint.SAVEBP_Checkpoint_C"))
      (Variables|Default|SetAs%20SAVEBP%20Checkpoint _returnvalue_3)))
  (bind _outactors (Actor|GetAllActorsOfClass "/Game/Blueprints/LevelDesign/BP_SaveGameCheckPoint.BP_SaveGameCheckPoint_C"))
  (bind _array_element (Utilities|Array|ForEachLoopwithBreak _outactors :!label _label)
    (:LoopBody
      (if (== (Variables|/Game/Blueprints/LevelDesign/BP_SaveGameCheckPoint.BP_SaveGameCheckPoint_C|GetCheckPoint_ID _array_element) (Variables|/Game/Blueprints/System/SaveGame/SAVEBP_Checkpoint.SAVEBP_Checkpoint_C|GetCheckpoint_ID (Variables|Default|GetAs%20SAVEBP%20Checkpoint)))
        (Utilities|FlowControl|Sequence
          (:then_0
            (goto _label Break))
          (:then_1
            (Default|EnableCheckPoint _array_element)))))))