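; Master collectible Blueprint that flies to the player and disappears when picked up.
; OnPickUpStart runs once, touches the game instance's currency view model (adding zero) and calls OnPickUpFinished before the movement starts.
; A timeline then pulls the actor toward player pawn 0 with exponentially accelerating interpolation, shrinking it each update and destroying it within close range.
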(event EventOnPickUpStart
  (bind _returnvalue (Game|GetGameInstance))
  (bind _asgi_my_game_instance (Utilities|Casting|CastToGI_MyGameInstance _returnvalue))
  (bind _vm_notplayerproperties (Variables|/Game/Blueprints/GI_MyGameInstance.GI_MyGameInstance_C|GetVM_NotPlayerProperties _asgi_my_game_instance))
  ;[1 1 1] need a check if has tag Player in the C++
  (Utilities|FlowControl|DoOnce false
    (:Completed
      (Variables|Default|SetTimeAtPickup (Utilities|Time|GetTimeSeconds))
      ;[1 1 1] WarnPickUpOnVM
      (Variables|/Script/MentoramaCPP5.NotPlayerProperties|SetCurrentCurrency _vm_notplayerproperties (+ 0 (Variables|/Script/MentoramaCPP5.NotPlayerProperties|GetCurrentCurrency _vm_notplayerproperties)))
      ;[1 1 1] sometimes this cast fails to find the player character when placed after the limeline so I placed it before
      (Class|CppCollectible|OnPickUpFinished)
      (Timeline|TML_MoveToCharacter Play
        (:Update
          (Transformation|SetActorLocation (Math|Interpolation|VInterpTo (Transformation|GetActorLocation) (Transformation|GetActorLocation (Game|Player|GetPlayerPawn 0)) (Utilities|Time|GetWorldDeltaSeconds) (+ (Math|Float|Power 2.0 (* (- (Utilities|Time|GetTimeSeconds) (Variables|Default|GetTimeAtPickup)) 5.0)) 1.0)) false false)
          (Transformation|SetActorRelativeScale3D (/ (Transformation|GetActorScale3D) 1.01))
          (if (<= (Math|Vector|Distance(Vector) (Transformation|GetActorLocation) (Transformation|GetActorLocation (Game|Player|GetPlayerPawn 0))) 5e+01)
            (Actor|DestroyActor)))))))

(fn ConstructionScript)