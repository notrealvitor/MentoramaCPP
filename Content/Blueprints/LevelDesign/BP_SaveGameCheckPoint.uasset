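; BP_SaveGameCheckPoint is a level checkpoint actor that saves progress when anything overlaps its sphere.
; On overlap it zeroes the Emitter material parameter on every checkpoint, then lights its own through a dynamic material instance created at BeginPlay.
; It then writes its location, level name and checkpoint ID into a new SAVEBP_Checkpoint object, saved to the single "Checkpoint" slot.
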(event OnComponentBeginOverlap(Sphere)
  (params (OverlappedComponent :type Primitive%20Component%20Object%20Reference) (OtherActor :type Actor%20Object%20Reference) (OtherComp :type Primitive%20Component%20Object%20Reference) (OtherBodyIndex :type Integer) (bFromSweep :type Boolean) (SweepResult :type Hit%20Result%20Structure%20%28by%20ref%29))
  (CallFunction|DisableAllCheckpoints)
  (CallFunction|EnableCheckPoint)
  (CallFunction|SavetoGameObject))

(event EventBeginPlay
  (bind _returnvalue (Rendering|Material|CreateDynamicMaterialInstance (Variables|Default|GetCube) 0 "/Game/Materials/MEI_SavePoint.MEI_SavePoint" "None" :!class /Script/Engine.PrimitiveComponent))
  (Variables|Default|SetREF_DynamicMaterial _returnvalue))

(fn ConstructionScript)

(fn EnableCheckPoint
  (Rendering|Material|SetScalarParameterValue (Variables|Default|GetREF_DynamicMaterial) "Emitter" 1.5e+02 :!class /Script/Engine.MaterialInstanceDynamic))

(fn DisableAllCheckpoints
  (bind _outactors (Actor|GetAllActorsOfClass "BP_SaveGameCheckPoint_C"))
  (for _array_element _outactors
    (Rendering|Material|SetScalarParameterValue (Variables|BP_SaveGameCheckPoint_C|GetREF_DynamicMaterial _array_element) "Emitter" 0.0 :!class /Script/Engine.MaterialInstanceDynamic)))

(fn SavetoGameObject
  (bind _returnvalue (SaveGame|CreateSaveGameObject "/Game/Blueprints/System/SaveGame/SAVEBP_Checkpoint.SAVEBP_Checkpoint_C"))
  (Variables|/Game/Blueprints/System/SaveGame/SAVEBP_Checkpoint.SAVEBP_Checkpoint_C|SetCharacterLocation _returnvalue (Transformation|GetActorLocation))
  (bind _returnvalue_2 (Game|GetCurrentLevelName true))
  (Variables|/Game/Blueprints/System/SaveGame/SAVEBP_Checkpoint.SAVEBP_Checkpoint_C|SetMapName _returnvalue _returnvalue_2)
  (Variables|/Game/Blueprints/System/SaveGame/SAVEBP_Checkpoint.SAVEBP_Checkpoint_C|SetCheckpoint_ID _returnvalue (Variables|Default|GetCheckPoint_ID))
  (SaveGame|SaveGametoSlot _returnvalue "Checkpoint"))