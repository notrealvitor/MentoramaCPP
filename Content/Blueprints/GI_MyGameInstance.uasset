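; Game instance that owns the global player-properties view model and handles score, level restart and quit confirmation.
; On Init it creates VM_PlayerProperties, registers it in the MVVM global view model collection and resets its currency, time and resource values.
; RestartGame resets those values and reopens the current level, while AddScore increments current currency.
; The quit request opens a confirm modal that either quits or removes itself and unbinds its events.
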(event Custom|OnNoButtonReleased_EventNo
  ;[0 0 0 1 42] QuitGame Modal
  (Widget|RemovefromParent (stale Custom|CreateQuitGameConfirmationModal _returnvalue))
  (CallFunction|UnbindAllfromModalConfirm (stale Custom|CreateQuitGameConfirmationModal _returnvalue)))

(event Custom|UnbindAllFromModalConfirm
  (params (Target :type WBP%20Modal%20Confirm%20Object%20Reference))
  ;[0 0 0 1 42] QuitGame Modal
  (EventDispatchers|UnbindallEventsfromOnNoButtonReleased Target)
  (EventDispatchers|UnbindallEventsfromOnYesButtonReleased Target))

(event Custom|RestartGame
  ;[0 0 0 1 42] RestartGame
  (Input|SetInputModeGameOnly (Game|GetPlayerController 0) false)
  (CallFunction|ResetVMPlayerProperties)
  (bind _returnvalue (Game|GetCurrentLevelName true))
  (Game|OpenLevel(byName) (Utilities|String|StringToName _returnvalue)))

(event Custom|CreateQuitGameConfirmationModal
  ;[0 0 0 1 42] QuitGame Modal
  (bind _returnvalue (UserInterface|CreateWidget "/Game/Blueprints/Widgets/WBP_ModalConfirm.WBP_ModalConfirm_C"))
  (UserInterface|Viewport|AddtoViewport _returnvalue 0)
  (EventDispatchers|AssignOnNoButtonReleased _returnvalue (delegate Custom|OnNoButtonReleased_EventNo))
  (EventDispatchers|AssignOnYesButtonReleased _returnvalue (delegate Custom|OnYesButtonReleased_EventYes)))

(event Custom|OnYesButtonReleased_EventYes
  ;[0 0 0 1 42] QuitGame Modal
  (Game|QuitGame 0 "Quit" false))

(event EventInit
  (bind _returnvalue (Game|ConstructObjectfromClass "/Game/Blueprints/Widgets/VisualModel/VM_PlayerProperties.VM_PlayerProperties_C"))
  (Variables|Default|SetVM_PlayerProperties _returnvalue)
  (Class|MVVMViewModelCollectionObject|AddViewModelInstance (Class|MVVMGameSubsystem|GetViewModelCollection (Subsystems|GetMVVMGameSubsystem)) (Utilities|Struct|MakeMVVMViewModelContext "/Game/Blueprints/Widgets/VisualModel/VM_PlayerProperties.VM_PlayerProperties_C" "VM_PlayerProperties") _returnvalue)
  (CallFunction|ResetVMPlayerProperties))

(fn ResetVMPlayerProperties
  (bind _vm_playerproperties (Variables|Default|GetVM_PlayerProperties))
  (Variables|/Game/Blueprints/Widgets/VisualModel/VM_PlayerProperties.VM_PlayerProperties_C|SetCurrentCurrency _vm_playerproperties 0)
  (Variables|/Game/Blueprints/Widgets/VisualModel/VM_PlayerProperties.VM_PlayerProperties_C|SetTotalCurrency _vm_playerproperties 0)
  (Variables|/Game/Blueprints/Widgets/VisualModel/VM_PlayerProperties.VM_PlayerProperties_C|SetTotalMapTime _vm_playerproperties 0.0)
  (Variables|/Game/Blueprints/Widgets/VisualModel/VM_PlayerProperties.VM_PlayerProperties_C|SetMapResource _vm_playerproperties 0)
  (Variables|/Game/Blueprints/Widgets/VisualModel/VM_PlayerProperties.VM_PlayerProperties_C|SetTimeTextColor _vm_playerproperties (Utilities|Struct|MakeSlateColor "(R=1.000000,G=1.000000,B=1.000000,A=1.000000)" "UseColor_Specified")))

(fn AddScore
  (params (Add :type Integer))
  (bind _vm_playerproperties (Variables|Default|GetVM_PlayerProperties))
  (Variables|/Game/Blueprints/Widgets/VisualModel/VM_PlayerProperties.VM_PlayerProperties_C|SetCurrentCurrency _vm_playerproperties (+ (Variables|/Game/Blueprints/Widgets/VisualModel/VM_PlayerProperties.VM_PlayerProperties_C|GetCurrentCurrency _vm_playerproperties) Add)))