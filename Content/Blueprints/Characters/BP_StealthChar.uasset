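; BP_StealthChar is a character Blueprint that shows a file-saved username on a text render component and creates the player HUD.
; BeginPlay loads any non-empty saved name, then creates WBP_PlayerHUD, passing in the VMPlayerProperties view model held by GI_MyGameInstance.
; The F key alternates between writing two hardcoded test usernames to file, reloading the displayed name after each write.
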(event EventBeginPlay
  (Utilities|FlowControl|Sequence
    (:then_0
      (CallFunction|LoadifValidUsername))
    (:then_1
      (bind _asgi_my_game_instance (Utilities|Casting|CastToGI_MyGameInstance (Game|GetGameInstance)))
      (Variables|Default|SetVM%20Player%20Properties (Variables|/Game/Blueprints/GI_MyGameInstance.GI_MyGameInstance_C|GetVM_PlayerProperties _asgi_my_game_instance))
      (bind _returnvalue (UserInterface|CreateWidget "/Game/Blueprints/Widgets/WBP_PlayerHUD.WBP_PlayerHUD_C" (Game|GetPlayerController 0) (Variables|/Game/Blueprints/GI_MyGameInstance.GI_MyGameInstance_C|GetVM_PlayerProperties _asgi_my_game_instance)))
      (bind _output_get (Variables|Default|SetVM_PlayerHUD _returnvalue))
      (UserInterface|Viewport|AddtoViewport _output_get 0))))

(event Input|KeyboardEvents|F
  (params (Key :type Key%20Structure :default "None"))
  (:Pressed
    (Utilities|FlowControl|FlipFlop
      (:A
        (Class|MentoramaHelpers|WriteUsernametoFile "usernameA")
        (CallFunction|LoadifValidUsername))
      (:B
        (Class|MentoramaHelpers|WriteUsernametoFile "usernameB")
        (CallFunction|LoadifValidUsername)))))

(fn ConstructionScript)

(fn LoadifValidUsername
  (bind _returnvalue (Class|MentoramaHelpers|ReadUsernamefromFile))
  (if (> (Utilities|String|Len _returnvalue) 0)
    (Rendering|Components|TextRender|SetText (Variables|Default|GetTextRender_Name) (Utilities|Text|ToText(String) _returnvalue))))