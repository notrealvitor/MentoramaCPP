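; AI character Blueprint with alert feedback, player tracking and a visible sight area.
; Events toggle an exclamation marker and run a timeline easing rotation toward a target; BeginPlay enables random direction when roaming.
; Sight points become actor-relative triangle data for a flat, translucent red procedural-mesh vision cone.
; SetHealthState maps health to state, but a constant comparison makes Recovery unreachable.
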(event Custom|LookAtPlayer
  (params (Target :type Vector%20%28by%20ref%29))
  ;[0 0 0 1 42] LookAtPlayer
  (Timeline|LookAtTimeline PlayFromStart
    (:Update
      (Transformation|SetActorRotation (Math|Rotator|Lerp(Rotator) (Transformation|GetActorRotation) (Math|Rotator|FindLookatRotation (Transformation|GetActorLocation) Target) 0.1 true)))))

(event Custom|SpotAlertVisibility
  (params (bNewVisibility :type Boolean))
  ;[0 0 0 1 42] Exclamation Spot Visibility
  (Rendering|SetVisibility (Variables|Default|GetExclamation) bNewVisibility false))

(event EventBeginPlay
  ;[0 0 0 1 42] BeginPlay
  (Utilities|FlowControl|Sequence
    (:then_1
      ;;[0.151 0 0] this could go in the C++
      (switch Utilities|FlowControl|Switch|SwitchonEState (Variables|/Script/MentoramaCPP5.AIBehaviourComponent|GetE_AIState (Variables|Default|GetAIBehaviour))
        (:Roaming
          (Variables|Default|SetRandomizeDirection true))))))

(fn ConstructionScript)

(fn PrintSelfAction
  (params (Action%20to%20Print :type String) (Duration :type Float%20%28double-precision%29))
  (Development|PrintString (Utilities|String|Append (Utilities|GetDisplayName self) " is " Action%20to%20Print) true true "(R=0.000000,G=0.660000,B=1.000000,A=1.000000)" Duration))

(fn SetHealthState
  (bind _s_aidata (Variables|Default|GetS_AIData))
  (if (>= (.health _s_aidata) 6e+01)
    (Variables|Default|SetE_HealthState "FullHealth")
    (return)
    (elif (<= (.health _s_aidata) 0.0)
      (Variables|Default|SetE_HealthState "Dead")
      (return)
      (elif (< 0.0 3e+01)
        (Variables|Default|SetE_HealthState "Endangered")
        (return)
        (elif (< (.health _s_aidata) 6e+01)
          (Variables|Default|SetE_HealthState "Recovery")
          (return))))))

(fn ConvertSightPointstoVertices
  (params (SightPoints :type Array%20of%20Vectors))
  (bind _returnvalue (Transformation|GetActorLocation))
  (bind _vertices (Variables|Default|GetVertices))
  (bind _returnvalue_2 (Utilities|Array|Length _vertices))
  (bind _returnvalue_3 (* _returnvalue_2 3))
  (Utilities|Array|SetArrayElem :TargetArray (Variables|Default|GetVertices))
  (for (_array_element _array_index) SightPoints
    (Utilities|Array|SetArrayElem (Variables|Default|GetVertices) _array_index (Math|Vector|MakeVector (- (.X (Math|Vector|BreakVector _array_element)) (.x _returnvalue)) (- (.Y (Math|Vector|BreakVector _array_element)) (.y _returnvalue)) 0.0)))
  (Utilities|Array|Resize (Variables|Default|GetTriangles) _returnvalue_3)
  (for _index (range 0 _returnvalue_3)
    (Utilities|Array|SetArrayElem (Variables|Default|GetTriangles) (* _index 3) 0)
    (Utilities|Array|SetArrayElem (Variables|Default|GetTriangles) (+ (* _index 3) 1) (+ _index 1))
    (Utilities|Array|SetArrayElem (Variables|Default|GetTriangles) (+ (+ (* _index 3) 1) 1) (+ (+ _index 1) 1)))
  (return (Variables|Default|GetVertices) (Variables|Default|GetTriangles)))

(fn BuildVisionCone
  (params (Vertices :type Array%20of%20Vectors) (Triangles :type Array%20of%20Integers))
  (bind _visioncone (Variables|Default|GetVisionCone))
  (Class|ProceduralMeshComponent|CreateMeshSectionLinearColor _visioncone 0 Vertices Triangles 0 0 0 0 0 0 0 false false)
  (Rendering|Material|SetMaterial _visioncone 0 "/Game/Materials/M_TransparentRed.M_TransparentRed")
  (Transformation|SetWorldRotation _visioncone "0, 0, 0" false false))